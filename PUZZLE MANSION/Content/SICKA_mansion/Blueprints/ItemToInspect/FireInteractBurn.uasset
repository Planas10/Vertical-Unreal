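; FireInteractBurn is an interactable fire that lets the player burn the item they are holding.
; GetInfoText shows a burn prompt when the held item has CanBeBurned set.
; On interact, it detaches that item, moves it to the Box component and clears the HUD text.
; After a short delay it destroys the item and calls BurnBook on the GameController game instance.
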(event EventBeginPlay)

(event Collision|EventActorBeginOverlap
  (params (OtherActor :type Actor%20Object%20Reference)))

(event EventTick
  (params (DeltaSeconds :type Float%20%28single-precision%29)))

(event EventInteractwith
  (params (PlayerCharacter :type BP%20Horror%20Character%20Object%20Reference))
  (bind _currentlyhelditem (Variables|/Game/SICKA_mansion/Blueprints/CharacterSystem/BP_HorrorCharacter.BP_HorrorCharacter_C|GetCurrentlyHeldItem PlayerCharacter))
  (Variables|Default|SetBurning _currentlyhelditem)
  (if (Utilities|IsValid _currentlyhelditem)
    (if (Variables|/Game/SICKA_mansion/Blueprints/ItemToInspect/BP_InteractObject_Master.BP_InteractObject_Master_C|GetcanBeBurned _currentlyhelditem)
      (Transformation|DetachFromActor _currentlyhelditem "KeepWorld" "KeepWorld" "KeepWorld")
      (Transformation|SetActorLocation (Variables|Default|GetBurning) (Transformation|GetWorldLocation (Variables|Default|GetBox)) false false)
      (Default|ClearInfoText (Variables|/Game/SICKA_mansion/Blueprints/CharacterSystem/BP_HorrorCharacter.BP_HorrorCharacter_C|GetPlayerHud PlayerCharacter))
      (Utilities|FlowControl|Delay 2.0)
      (Actor|DestroyActor (Variables|Default|GetBurning))
      (bind _asgame_controller (Utilities|Casting|CastToGameController (Game|GetGameInstance)))
      (Default|BurnBook _asgame_controller))))

(fn ConstructionScript)

(fn GetInfoText
  (params (Player :type BP%20Horror%20Character%20Object%20Reference))
  (bind _currentlyhelditem (Variables|/Game/SICKA_mansion/Blueprints/CharacterSystem/BP_HorrorCharacter.BP_HorrorCharacter_C|GetCurrentlyHeldItem Player))
  (if (Utilities|IsValid _currentlyhelditem)
    (if (Variables|/Game/SICKA_mansion/Blueprints/ItemToInspect/BP_InteractObject_Master.BP_InteractObject_Master_C|GetcanBeBurned _currentlyhelditem)
      (return "Burn Item")
      (else
        (return "")))))