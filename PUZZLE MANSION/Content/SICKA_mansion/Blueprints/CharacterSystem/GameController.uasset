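; GameController tracks progression through the mansion's three-stage puzzle chain: burning books, activating globes and cooking.
; Each action plays a sound and increments a counter that starts the next stage at its threshold, with CurrentPuzzle guarding against repeat starts.
; Stage starts make GloboTerraqueo globes glow, then unhide "Cook"-tagged actors.
; Completing cooking rotates "Puerta"-tagged actors to open the final door, without a stage guard.
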(fn BurnBook
  (bind _burnedbooks (Variables|Default|GetBurnedBooks))
  (Audio|PlaySound2D "/Game/SICKA_mansion/Sound/99506-Torch_pass_by_whoosh_fast_03-SFXBible-ss00747.99506-Torch_pass_by_whoosh_fast_03-SFXBible-ss00747" 1.0 1.0 0.0 0 0)
  (Math|Integer|IncrementInt _burnedbooks
    (:%20%20
      (if (>= _burnedbooks (Variables|Default|GetneededBurnedBooks))
        (CallFunction|Puzzle2Start)))))

(fn Puzzle2Start
  (if (< (Variables|Default|GetCurrentPuzzle) 2)
    (Variables|Default|SetCurrentPuzzle 2)
    (Audio|PlaySound2D "/Game/SICKA_mansion/Sound/223130-transitional-confirms-21.223130-transitional-confirms-21" 1.0 1.0 0.0 0 0)
    (bind _outactors (Actor|GetAllActorsOfClass "/Game/SICKA_mansion/Blueprints/CharacterSystem/GloboTerraqueo.GloboTerraqueo_C"))
    (for _array_element _outactors
      (Default|ActivateGlow _array_element))))

(fn ActivateGlobe
  (bind _currentglobes (Variables|Default|GetcurrentGlobes))
  (Audio|PlaySound2D "/Game/SICKA_mansion/Sound/492560-glass-tick-navigation-10.492560-glass-tick-navigation-10" 1.0 1.0 0.0 0 0)
  (Math|Integer|IncrementInt _currentglobes
    (:%20%20
      (if (>= _currentglobes (Variables|Default|GetneededGlobes))
        (CallFunction|Puzzle3Start)))))

(fn Puzzle3Start
  (if (< (Variables|Default|GetCurrentPuzzle) 3)
    (Variables|Default|SetCurrentPuzzle 3)
    (Audio|PlaySound2D "/Game/SICKA_mansion/Sound/223130-transitional-confirms-21.223130-transitional-confirms-21" 1.0 1.0 0.0 0 0)
    (bind _outactors (Actor|GetAllActorswithTag "Cook"))
    (for _array_element _outactors
      (Rendering|SetActorHiddenInGame _array_element false))))

(fn OpenFinalDoor
  (bind _outactors (Actor|GetAllActorswithTag "Puerta"))
  (for _array_element _outactors
    (Audio|PlaySound2D "/Game/SICKA_mansion/Sound/120703-Door_creaking_with_short_ticks_and_reverb_2.120703-Door_creaking_with_short_ticks_and_reverb_2" 1.0 1.0 0.0 0 0)
    (Transformation|SetActorRotation _array_element "0.000000,-19.999877,0.000000")))

(fn Cook
  (bind _cooked (Variables|Default|Getcooked))
  (Audio|PlaySound2D "/Game/SICKA_mansion/Sound/90888-Swallow_water_big_gulp-BLASTWAVEFX-25468.90888-Swallow_water_big_gulp-BLASTWAVEFX-25468" 1.0 1.0 0.0 0 0)
  (Math|Integer|IncrementInt _cooked
    (:%20%20
      (if (>= _cooked (Variables|Default|GetneededForCook))
        (CallFunction|OpenFinalDoor)))))