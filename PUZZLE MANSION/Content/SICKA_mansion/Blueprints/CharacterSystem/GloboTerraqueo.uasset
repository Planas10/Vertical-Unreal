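; GloboTerraqueo is an interactable globe that the player can activate.
; Interacting hides its outline and calls ActivateGlobe on the GameController game instance.
; ActivateGlow shows the outline, and GetInfoText returns an "Activate Globe" prompt unless BoolUsed is true.
; Interaction sets BoolUsed to false, so nothing in these graphs marks the globe as used.
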(event EventBeginPlay)

(event Collision|EventActorBeginOverlap
  (params (OtherActor :type Actor%20Object%20Reference)))

(event EventTick
  (params (DeltaSeconds :type Float%20%28single-precision%29)))

(event EventInteractwith
  (params (PlayerCharacter :type BP%20Horror%20Character%20Object%20Reference))
  (Rendering|SetVisibility (Variables|Default|GetOutline) false false)
  (Variables|Default|Setbool%20used false)
  (bind _asgame_controller (Utilities|Casting|CastToGameController (Game|GetGameInstance)))
  (Default|ActivateGlobe _asgame_controller))

(fn ConstructionScript)

(fn ActivateGlow
  (Rendering|SetVisibility (Variables|Default|GetOutline) true false))

(fn GetInfoText
  (params (Player :type BP%20Horror%20Character%20Object%20Reference))
  (if (Variables|Default|Getbool%20used)
    (return "")
    (else
      (return "Activate Globe"))))